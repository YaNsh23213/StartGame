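; BP_NPTalent is an NPC actor that shows its Widget component only while the player's pawn is nearby.
; On BeginPlay it hides the widget, waits through a long fixed delay, then starts a looping one-second timer that calls CheckVisible.
; CheckVisible compares the distance to the first player's pawn against a fixed radius and toggles visibility only when the state must change, avoiding per-Tick checks.
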(event `self.ReceiveBeginPlay`
  (`SceneComponent.SetVisibility` (`self.Widget`) false false)
  (`KismetSystemLibrary.Delay` 39.0)
  (`KismetSystemLibrary.K2_SetTimer` null "CheckVisible" 1.0 true))

(event `self.ReceiveTick`
  (params (DeltaSeconds :type "Float (single-precision)")))

(fn `CheckVisible`
  (bind _widget (`self.Widget`))
  (bind _returnvalue (`WidgetComponent.IsWidgetVisible` _widget))
  (if (< (`self.GetDistanceTo` self (`Controller.K2_GetPawn` (`GameplayStatics.GetPlayerController` 0))) 3000.0)
    (if (not _returnvalue)
      (`SceneComponent.SetVisibility` _widget true false))
    (elif _returnvalue
      (`SceneComponent.SetVisibility` _widget false false))))

(fn `UserConstructionScript`)